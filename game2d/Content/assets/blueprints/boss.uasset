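; Boss actor that patrols back and forth along the world X axis, attacks the player and can be defeated with fireballs.
; Tick moves it by a signed Speed, reversing direction at hard-coded world X bounds.
; Box1 spawns a Boss_atack just below the boss when a "player"-tagged component enters it.
; Box decrements Life on "fireball"-tagged overlaps, destroying the boss at zero and printing a Portuguese victory message.
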(event `self.ReceiveTick`
  (params (DeltaSeconds :type "Float (single-precision)"))
  (bind _x (.x (`self.K2_GetActorLocation`)))
  (`self.K2_AddActorWorldOffset` (`KismetMathLibrary.MakeVector` (* DeltaSeconds (`self.speed`))))
  (if (>= _x 220.0)
    (set `self.speed` -200.0)
    (elif (<= _x -230.0)
      (set `self.speed` 200.0))))

(event `self.Box1.OnComponentBeginOverlap`
  (params (OverlappedComponent :type "PrimitiveComponent Object Reference") (OtherActor :type "Actor Object Reference") (OtherComp :type "PrimitiveComponent Object Reference") (OtherBodyIndex :type Integer) (bFromSweep :type Boolean) (SweepResult :type "HitResult Structure (by ref)"))
  (if (`ActorComponent.ComponentHasTag` OtherComp "player")
    (`|SpawnActorFromClass` "/Game/assets/blueprints/boss_atack.boss_atack_C" (`KismetMathLibrary.MakeTransform` (`KismetMathLibrary.MakeVector` (.x (`self.K2_GetActorLocation`)) (.y (`self.K2_GetActorLocation`)) (+ (.z (`self.K2_GetActorLocation`)) -50.0))) "Undefined" "OverrideRootScale" null null)))

(event `self.Box.OnComponentBeginOverlap`
  (params (OverlappedComponent :type "PrimitiveComponent Object Reference") (OtherActor :type "Actor Object Reference") (OtherComp :type "PrimitiveComponent Object Reference") (OtherBodyIndex :type Integer) (bFromSweep :type Boolean) (SweepResult :type "HitResult Structure (by ref)"))
  (if (`ActorComponent.ComponentHasTag` OtherComp "fireball")
    (bind _output_get (set `self.life` (- (`self.life`) 1.0)))
    (if (== _output_get 0.0)
      (`self.K2_DestroyActor`)
      (`KismetSystemLibrary.PrintString` "vc venceu"))))

(fn `UserConstructionScript`)