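; Falling block actor that drops straight down at a constant speed until it rests on something.
; Tick offsets it downward each frame without sweep, stopping while the IsOverlapping flag is set.
; Its Box component's begin and end overlap events set and clear that flag, ignoring components tagged boss, seeker or bossatack.
; The flag is a single boolean, so ending any counted overlap resumes the fall.
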(event `self.ReceiveBeginPlay`)

(event `self.ReceiveActorBeginOverlap`
  (params (OtherActor :type "Actor Object Reference")))

(event `self.ReceiveTick`
  (params (DeltaSeconds :type "Float (single-precision)"))
  (if (`self.isOverlapping`)
    (set `self.speed` 0.0)
    (else
      (set `self.speed` -400.0)))
  (`self.K2_AddActorWorldOffset` (`KismetMathLibrary.MakeVector` 0.0 0.0 (* DeltaSeconds (`self.speed`)))))

(event `self.Box.OnComponentBeginOverlap`
  (params (OverlappedComponent :type "PrimitiveComponent Object Reference") (OtherActor :type "Actor Object Reference") (OtherComp :type "PrimitiveComponent Object Reference") (OtherBodyIndex :type Integer) (bFromSweep :type Boolean) (SweepResult :type "HitResult Structure (by ref)"))
  (if (`ActorComponent.ComponentHasTag` OtherComp "boss")
    _
    (elif (`ActorComponent.ComponentHasTag` OtherComp "seeker")
      _
      (elif (not (`ActorComponent.ComponentHasTag` OtherComp "bossatack"))
        (set `self.isOverlapping` true)))))

(event `self.Box.OnComponentEndOverlap`
  (params (OverlappedComponent :type "PrimitiveComponent Object Reference") (OtherActor :type "Actor Object Reference") (OtherComp :type "PrimitiveComponent Object Reference") (OtherBodyIndex :type Integer))
  (if (`ActorComponent.ComponentHasTag` OtherComp "boss")
    _
    (elif (`ActorComponent.ComponentHasTag` OtherComp "seeker")
      _
      (elif (not (`ActorComponent.ComponentHasTag` OtherComp "bossatack"))
        (set `self.isOverlapping` false)))))

(fn `UserConstructionScript`)