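; Fireball projectile that travels along world Z and destroys falling blocks it hits.
; Tick offsets it by Speed scaled by delta time, without sweep, so hits rely on the Box overlap event.
; Components tagged "kill" or "block" destroy their owning fall_block and the fireball.
; A "boss" tag destroys only the fireball, with no damage applied here.
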(event `self.ReceiveActorBeginOverlap`
  (params (OtherActor :type "Actor Object Reference")))

(event `self.ReceiveTick`
  (params (DeltaSeconds :type "Float (single-precision)"))
  (`self.K2_AddActorWorldOffset` (`KismetMathLibrary.MakeVector` 0.0 0.0 (* DeltaSeconds (`self.speed`)))))

(event `self.Box.OnComponentBeginOverlap`
  (params (OverlappedComponent :type "PrimitiveComponent Object Reference") (OtherActor :type "Actor Object Reference") (OtherComp :type "PrimitiveComponent Object Reference") (OtherBodyIndex :type Integer) (bFromSweep :type Boolean) (SweepResult :type "HitResult Structure (by ref)"))
  (if (`ActorComponent.ComponentHasTag` OtherComp "kill")
    (bind _asfall_block (cast `/Game/assets/blueprints/fall_block` OtherActor))
    (`self.K2_DestroyActor` _asfall_block)
    (`self.K2_DestroyActor` :!label _label)
    (elif (`ActorComponent.ComponentHasTag` OtherComp "block")
      (bind _asfall_block_2 (cast `/Game/assets/blueprints/fall_block` OtherActor))
      (`self.K2_DestroyActor` _asfall_block_2)
      (goto _label)
      (elif (`ActorComponent.ComponentHasTag` OtherComp "boss")
        (goto _label)))))

(fn `UserConstructionScript`)