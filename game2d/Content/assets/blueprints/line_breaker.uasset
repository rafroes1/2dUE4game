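; Line-breaker actor that detects falling blocks across fourteen box triggers and destroys them, apparently for clearing rows.
; Each box overlap with a "kill"-tagged component inserts true into Collisions (never reset) and stores the fall_block.
; Tick walks the first five flags, destroying each block until one is false, without requiring all five.
; Later boxes' blocks are stored but never destroyed; ClearBlock duplicates Tick's chain and is only called from unconnected nodes.
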(event `self.ReceiveTick`
  (params (DeltaSeconds :type "Float (single-precision)"))
  (bind _collisions (`self.collisions`))
  (if (`|GetArrayItem` _collisions)
    (`self.K2_DestroyActor` (`self.block0`))
    (if (`|GetArrayItem` _collisions 1)
      (`self.K2_DestroyActor` (`self.block1`))
      (if (`|GetArrayItem` _collisions 2)
        (`self.K2_DestroyActor` (`self.block2`))
        (if (`|GetArrayItem` _collisions 3)
          (`self.K2_DestroyActor` (`self.block3`))
          (if (`|GetArrayItem` (`self.collisions`) 4)
            (`self.K2_DestroyActor` (`self.block4`))))))))

(event `self.Box00.OnComponentBeginOverlap`
  (params (OverlappedComponent :type "PrimitiveComponent Object Reference") (OtherActor :type "Actor Object Reference") (OtherComp :type "PrimitiveComponent Object Reference") (OtherBodyIndex :type Integer) (bFromSweep :type Boolean) (SweepResult :type "HitResult Structure (by ref)"))
  (if (`ActorComponent.ComponentHasTag` OtherComp "kill")
    (`KismetArrayLibrary.Array_Insert` (`self.collisions`) true)
    (bind _asfall_block (cast `/Game/assets/blueprints/fall_block` OtherActor))
    (set `self.block0` _asfall_block)))

(event `self.Box01.OnComponentBeginOverlap`
  (params (OverlappedComponent :type "PrimitiveComponent Object Reference") (OtherActor :type "Actor Object Reference") (OtherComp :type "PrimitiveComponent Object Reference") (OtherBodyIndex :type Integer) (bFromSweep :type Boolean) (SweepResult :type "HitResult Structure (by ref)"))
  (if (`ActorComponent.ComponentHasTag` OtherComp "kill")
    (`KismetArrayLibrary.Array_Insert` (`self.collisions`) true 1)
    (bind _asfall_block (cast `/Game/assets/blueprints/fall_block` OtherActor))
    (set `self.block1` _asfall_block)))

(event `self.Box02.OnComponentBeginOverlap`
  (params (OverlappedComponent :type "PrimitiveComponent Object Reference") (OtherActor :type "Actor Object Reference") (OtherComp :type "PrimitiveComponent Object Reference") (OtherBodyIndex :type Integer) (bFromSweep :type Boolean) (SweepResult :type "HitResult Structure (by ref)"))
  (if (`ActorComponent.ComponentHasTag` OtherComp "kill")
    (`KismetArrayLibrary.Array_Insert` (`self.collisions`) true 2)
    (bind _asfall_block (cast `/Game/assets/blueprints/fall_block` OtherActor))
    (set `self.block2` _asfall_block)))

(event `self.Box03.OnComponentBeginOverlap`
  (params (OverlappedComponent :type "PrimitiveComponent Object Reference") (OtherActor :type "Actor Object Reference") (OtherComp :type "PrimitiveComponent Object Reference") (OtherBodyIndex :type Integer) (bFromSweep :type Boolean) (SweepResult :type "HitResult Structure (by ref)"))
  (if (`ActorComponent.ComponentHasTag` OtherComp "kill")
    (`KismetArrayLibrary.Array_Insert` (`self.collisions`) true 3)
    (bind _asfall_block (cast `/Game/assets/blueprints/fall_block` OtherActor))
    (set `self.block3` _asfall_block)))

(event `self.Box04.OnComponentBeginOverlap`
  (params (OverlappedComponent :type "PrimitiveComponent Object Reference") (OtherActor :type "Actor Object Reference") (OtherComp :type "PrimitiveComponent Object Reference") (OtherBodyIndex :type Integer) (bFromSweep :type Boolean) (SweepResult :type "HitResult Structure (by ref)"))
  (if (`ActorComponent.ComponentHasTag` OtherComp "kill")
    (`KismetArrayLibrary.Array_Insert` (`self.collisions`) true 4)
    (bind _asfall_block (cast `/Game/assets/blueprints/fall_block` OtherActor))
    (set `self.block4` _asfall_block)))

(event `self.Box05.OnComponentBeginOverlap`
  (params (OverlappedComponent :type "PrimitiveComponent Object Reference") (OtherActor :type "Actor Object Reference") (OtherComp :type "PrimitiveComponent Object Reference") (OtherBodyIndex :type Integer) (bFromSweep :type Boolean) (SweepResult :type "HitResult Structure (by ref)"))
  (if (`ActorComponent.ComponentHasTag` OtherComp "kill")
    (`KismetArrayLibrary.Array_Insert` (`self.collisions`) true 5)
    (bind _asfall_block (cast `/Game/assets/blueprints/fall_block` OtherActor))
    (`KismetArrayLibrary.Array_Insert` (`self.blocks`) _asfall_block 5)))

(event `self.Box06.OnComponentBeginOverlap`
  (params (OverlappedComponent :type "PrimitiveComponent Object Reference") (OtherActor :type "Actor Object Reference") (OtherComp :type "PrimitiveComponent Object Reference") (OtherBodyIndex :type Integer) (bFromSweep :type Boolean) (SweepResult :type "HitResult Structure (by ref)"))
  (if (`ActorComponent.ComponentHasTag` OtherComp "kill")
    (`KismetArrayLibrary.Array_Insert` (`self.collisions`) true 6)
    (bind _asfall_block (cast `/Game/assets/blueprints/fall_block` OtherActor))
    (`KismetArrayLibrary.Array_Insert` (`self.blocks`) _asfall_block 6)))

(event `self.Box07.OnComponentBeginOverlap`
  (params (OverlappedComponent :type "PrimitiveComponent Object Reference") (OtherActor :type "Actor Object Reference") (OtherComp :type "PrimitiveComponent Object Reference") (OtherBodyIndex :type Integer) (bFromSweep :type Boolean) (SweepResult :type "HitResult Structure (by ref)"))
  (if (`ActorComponent.ComponentHasTag` OtherComp "kill")
    (`KismetArrayLibrary.Array_Insert` (`self.collisions`) true 7)
    (bind _asfall_block (cast `/Game/assets/blueprints/fall_block` OtherActor))
    (`KismetArrayLibrary.Array_Insert` (`self.blocks`) _asfall_block 7)))

(event `self.Box08.OnComponentBeginOverlap`
  (params (OverlappedComponent :type "PrimitiveComponent Object Reference") (OtherActor :type "Actor Object Reference") (OtherComp :type "PrimitiveComponent Object Reference") (OtherBodyIndex :type Integer) (bFromSweep :type Boolean) (SweepResult :type "HitResult Structure (by ref)"))
  (if (`ActorComponent.ComponentHasTag` OtherComp "kill")
    (`KismetArrayLibrary.Array_Insert` (`self.collisions`) true 8)
    (bind _asfall_block (cast `/Game/assets/blueprints/fall_block` OtherActor))
    (`KismetArrayLibrary.Array_Insert` (`self.blocks`) _asfall_block 8)))

(event `self.Box09.OnComponentBeginOverlap`
  (params (OverlappedComponent :type "PrimitiveComponent Object Reference") (OtherActor :type "Actor Object Reference") (OtherComp :type "PrimitiveComponent Object Reference") (OtherBodyIndex :type Integer) (bFromSweep :type Boolean) (SweepResult :type "HitResult Structure (by ref)"))
  (if (`ActorComponent.ComponentHasTag` OtherComp "kill")
    (`KismetArrayLibrary.Array_Insert` (`self.collisions`) true 9)
    (bind _asfall_block (cast `/Game/assets/blueprints/fall_block` OtherActor))
    (`KismetArrayLibrary.Array_Insert` (`self.blocks`) _asfall_block 9)))

(event `self.Box10.OnComponentBeginOverlap`
  (params (OverlappedComponent :type "PrimitiveComponent Object Reference") (OtherActor :type "Actor Object Reference") (OtherComp :type "PrimitiveComponent Object Reference") (OtherBodyIndex :type Integer) (bFromSweep :type Boolean) (SweepResult :type "HitResult Structure (by ref)"))
  (if (`ActorComponent.ComponentHasTag` OtherComp "kill")
    (`KismetArrayLibrary.Array_Insert` (`self.collisions`) true 10)
    (bind _asfall_block (cast `/Game/assets/blueprints/fall_block` OtherActor))
    (`KismetArrayLibrary.Array_Insert` (`self.blocks`) _asfall_block 10)))

(event `self.Box11.OnComponentBeginOverlap`
  (params (OverlappedComponent :type "PrimitiveComponent Object Reference") (OtherActor :type "Actor Object Reference") (OtherComp :type "PrimitiveComponent Object Reference") (OtherBodyIndex :type Integer) (bFromSweep :type Boolean) (SweepResult :type "HitResult Structure (by ref)"))
  (if (`ActorComponent.ComponentHasTag` OtherComp "kill")
    (`KismetArrayLibrary.Array_Insert` (`self.collisions`) true 11)
    (bind _asfall_block (cast `/Game/assets/blueprints/fall_block` OtherActor))
    (`KismetArrayLibrary.Array_Insert` (`self.blocks`) _asfall_block 11)))

(event `self.Box12.OnComponentBeginOverlap`
  (params (OverlappedComponent :type "PrimitiveComponent Object Reference") (OtherActor :type "Actor Object Reference") (OtherComp :type "PrimitiveComponent Object Reference") (OtherBodyIndex :type Integer) (bFromSweep :type Boolean) (SweepResult :type "HitResult Structure (by ref)"))
  (if (`ActorComponent.ComponentHasTag` OtherComp "kill")
    (`KismetArrayLibrary.Array_Insert` (`self.collisions`) true 12)
    (bind _asfall_block (cast `/Game/assets/blueprints/fall_block` OtherActor))
    (`KismetArrayLibrary.Array_Insert` (`self.blocks`) _asfall_block 12)))

(event `self.Box13.OnComponentBeginOverlap`
  (params (OverlappedComponent :type "PrimitiveComponent Object Reference") (OtherActor :type "Actor Object Reference") (OtherComp :type "PrimitiveComponent Object Reference") (OtherBodyIndex :type Integer) (bFromSweep :type Boolean) (SweepResult :type "HitResult Structure (by ref)"))
  (if (`ActorComponent.ComponentHasTag` OtherComp "kill")
    (`KismetArrayLibrary.Array_Insert` (`self.collisions`) true 13)
    (bind _asfall_block (cast `/Game/assets/blueprints/fall_block` OtherActor))
    (`KismetArrayLibrary.Array_Insert` (`self.blocks`) _asfall_block 13)))

(fn `clearBlock`
  (bind _collisions (`self.collisions`))
  (if (`|GetArrayItem` _collisions)
    (`self.K2_DestroyActor` (`self.block0`))
    (if (`|GetArrayItem` _collisions 1)
      (`self.K2_DestroyActor` (`self.block1`))
      (if (`|GetArrayItem` _collisions 2)
        (`self.K2_DestroyActor` (`self.block2`))
        (if (`|GetArrayItem` _collisions 3)
          (`self.K2_DestroyActor` (`self.block3`))
          (if (`|GetArrayItem` (`self.collisions`) 4)
            (`self.K2_DestroyActor` (`self.block4`))))))))

(fn `UserConstructionScript`)