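; Spawner actor that drops blocks, fireballs, lives and bosses into the block game at random horizontal positions.
; It binds to the game mode's start and end events to run or clear a looping Spawn timer.
; Each spawn picks one of fourteen evenly spaced X slots at the actor's Y and Z, with a weighted random type favoring blocks.
; Spawning a block also increments the score shown on the player character's GameWidget.
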(event `self.ReceiveBeginPlay`
  (bind _asblocksgamemode (cast `/Game/assets/blueprints/blocksgamemode` (`GameplayStatics.GetGameMode`)))
  (add `/Game/assets/blueprints/blocksgamemode.gameStarted` _asblocksgamemode (delegate `callStart`))
  (add `/Game/assets/blueprints/blocksgamemode.gameEnded` _asblocksgamemode (delegate `callEnd`)))

(event `callStart`
  (`self.start`))

(event `callEnd`
  (`self.stop`))

(event `self.ReceiveTick`
  (params (DeltaSeconds :type "Float (single-precision)")))

(fn `setX`
  (returns (x :type Integer) (Output_Get :type Integer))
  (bind _xlocation (`self.xLocation`))
  (switch `int` (`KismetMathLibrary.RandomIntegerInRange` 1 14)
    (:`1`
      (set `self.xLocation` -218))
    (:`2`
      (set `self.xLocation` -185))
    (:`3`
      (set `self.xLocation` -152))
    (:`4`
      (set `self.xLocation` -119))
    (:`5`
      (set `self.xLocation` -86))
    (:`6`
      (set `self.xLocation` -53))
    (:`7`
      (set `self.xLocation` -20))
    (:`8`
      (set `self.xLocation` 13))
    (:`9`
      (set `self.xLocation` 46))
    (:`10`
      (set `self.xLocation` 79))
    (:`11`
      (set `self.xLocation` 112))
    (:`12`
      (set `self.xLocation` 145))
    (:`13`
      (set `self.xLocation` 178))
    (:`14`
      (set `self.xLocation` 211)))
  (return _xlocation _xlocation))

(fn `spawn`
  (bind _x (`self.setX`))
  (switch `int` (`KismetMathLibrary.RandomIntegerInRange` 0 9)
    (:`0`
      (bind _returnvalue (`KismetMathLibrary.MakeTransform` (`KismetMathLibrary.MakeVector` (`KismetMathLibrary.Conv_IntToDouble` _x) (.y (`self.K2_GetActorLocation`)) (.z (`self.K2_GetActorLocation`)))))
      (`|SpawnActorFromClass` (`self.blockTemplate`) _returnvalue "AlwaysSpawn" "OverrideRootScale" null null :!label _label)
      (bind _output_get (set `self.score` (+ (`self.score`) 1)))
      (`/Game/assets/umg/startWidget.addScore` (`self.gameWidget`) _output_get))
    (:`1`
      (goto _label))
    (:`2`
      (goto _label))
    (:`3`
      (goto _label))
    (:`4`
      (goto _label))
    (:`5`
      (goto _label))
    (:`6`
      (goto _label))
    (:`7`
      (`|SpawnActorFromClass` (`self.fireballTemplate`) _returnvalue "AlwaysSpawn" "OverrideRootScale" null null))
    (:`8`
      (`|SpawnActorFromClass` (`self.lifeTemplate`) _returnvalue "AlwaysSpawn" "OverrideRootScale" null null))
    (:`9`
      (`|SpawnActorFromClass` (`self.bossTemplate`) _returnvalue "AlwaysSpawn" "OverrideRootScale" null null))))

(fn `start`
  (`self.spawn`)
  (bind _returnvalue (`KismetSystemLibrary.K2_SetTimer` null "spawn" (`self.spawnInterval`) true))
  (set `self.timerHandle` _returnvalue)
  (bind _ascharacter (cast `/Game/assets/blueprints/character` (`GameplayStatics.GetPlayerPawn` 0)))
  (set `self.gameWidget` (`/Game/assets/blueprints/character.gameWidget` _ascharacter)))

(fn `stop`
  (`KismetSystemLibrary.K2_ClearAndInvalidateTimerHandle` (`self.timerHandle`)))

(fn `UserConstructionScript`)